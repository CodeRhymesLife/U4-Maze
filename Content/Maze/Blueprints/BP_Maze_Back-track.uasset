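; Maze generator Blueprint that builds a bordered grid maze in the construction script using a depth-first backtracking algorithm.
; From a start tile, it takes seeded random two-tile steps, recording path and bridge tiles, then backtracks at dead ends, converting bridges to path.
; Unused cells become walls, with fixed shares of sand and bush variants assigned by index.
; Tile indices map to grid positions for instanced border, floor and wall meshes.
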(event EventBeginPlay)

(event EventActorBeginOverlap
  (params (OtherActor :type Actor%20Object%20Reference)))

(event EventTick
  (params (DeltaSeconds :type Float%20%28single-precision%29)))

(fn ConstructionScript
  (CallFunction|PopulateBoarders (Variables|Default|GetSize) (Variables|Default|GetBoarderTiles))
  (if (Variables|Default|GetShowBoarder?)
    ;[1 1 1] Create Boarder Tiles
    (Utilities|SpawnInstances (Variables|Default|GetBoarderTiles) (Variables|Default|GetSize) (Variables|Default|GetTileSize) "1.000000,1.000000,2.000000" (Variables|Default|GetBoarder)
      (:Finished
        _)))
  (if (Variables|Default|GetShowMaze)
    (CallFunction|SetInitialTile)
    (while (Variables|Default|GetbCurrentFreeSide?) :!label _label
      (CallFunction|PickNearbyTile))
    (Utilities|Array|Add (Variables|Default|GetCheckedTiles) (Variables|Default|GetCurrentTile))
    (CallFunction|BackTrack)
    (Utilities|ConvertLastBridge
      (:BridgesLeft
        (goto _label))
      (:No%20BridgesLeft
        ;[1 1 1] Create Path Tiles
        (Utilities|SpawnInstances (Variables|Default|GetPathTiles) (Variables|Default|GetSize) (Variables|Default|GetTileSize) "1.000000,1.000000,0.125000" (Variables|Default|GetFloor)
          (:Finished
            (CallFunction|PopulateWalls)
            ;[1 1 1] Create Walls
            (Utilities|SpawnInstances (Variables|Default|GetNormalWallTiles) (Variables|Default|GetSize) (Variables|Default|GetTileSize) "1.000000,1.000000,1.000000" (Variables|Default|GetNoramlWall)
              (:Finished
                (Utilities|SpawnInstances (Variables|Default|GetSandWallTiles) (Variables|Default|GetSize) (Variables|Default|GetTileSize) "1.000000,1.000000,1.000000" (Variables|Default|GetSandWall)
                  (:Finished
                    (Utilities|SpawnInstances (Variables|Default|GetBushWallTiles) (Variables|Default|GetSize) (Variables|Default|GetTileSize) "1.000000,1.000000,1.000000" (Variables|Default|GetBushWall))))))))))))

(fn PopulateBoarders
  (params (Size :type Integer) (BorderArray :type Array%20of%20Integers))
  (LocalVariables|SetL_Size Size)
  ;[1 1 1] North Boarder
  (for _index (range 0 (- (LocalVariables|GetL_Size) 1))
    (Utilities|Array|Add BorderArray _index))
  ;[1 1 1] East Boarder
  (for _index_2 (range 1 (- (LocalVariables|GetL_Size) 2))
    (Utilities|Array|Add BorderArray (+ (* _index_2 (LocalVariables|GetL_Size)) (- (LocalVariables|GetL_Size) 1))))
  ;[1 1 1] South Boarder
  (for _index_3 (range 1 (LocalVariables|GetL_Size))
    (Utilities|Array|Add BorderArray (+ (- _index_3 1) (* (LocalVariables|GetL_Size) (- (LocalVariables|GetL_Size) 1)))))
  ;[1 1 1] West Boarder
  (for _index_4 (range 1 (- (LocalVariables|GetL_Size) 2))
    (Utilities|Array|Add BorderArray (* _index_4 (LocalVariables|GetL_Size)))))

(fn SetInitialTile
  (Variables|Default|SetCurrentTile (+ (Variables|Default|GetSize) 1))
  (Utilities|Array|Add (Variables|Default|GetPathTiles) (Variables|Default|GetCurrentTile)))

(fn AddBridge&PathTile
  (params (PathTile :type Integer) (BridgeTile :type Integer))
  (Utilities|Array|Add (Variables|Default|GetPathTiles) PathTile)
  (Variables|Default|SetCurrentTile PathTile)
  (Utilities|Array|Add (Variables|Default|GetBridgeTiles) BridgeTile))

(fn PickNearbyTile
  (bind _currenttile (Variables|Default|GetCurrentTile))
  (bind _size (Variables|Default|GetSize))
  (bind _currenttile_2 (Variables|Default|GetCurrentTile))
  (bind _currenttile_3 (Variables|Default|GetCurrentTile))
  (bind _size_2 (Variables|Default|GetSize))
  (bind _currenttile_4 (Variables|Default|GetCurrentTile))
  (bind (_btileinarray _pathtile _bridgetile) (Utilities|CheckNorthTile _currenttile _size true))
  (bind (_btileinarray_2 _pathtile_2 _bridgetile_2) (Utilities|CheckEastTile _currenttile_2 true))
  (bind (_btileinarray_3 _pathtile_3 _bridgetile_3) (Utilities|CheckNorthTile _currenttile_3 _size_2 false))
  (bind (_btileinarray_4 _pathtile_4 _bridgetile_4) (Utilities|CheckEastTile _currenttile_4 false))
  (switch int (Math|Random|RandomIntegerinRangefromStream 0 3 (Variables|Default|GetRandomStream))
    (:0
      ;[1 1 1] North
      (if _btileinarray_3 :!label _label
        (Utilities|CycleCounter (LocalVariables|GetL_CycleCounter) 4
          (:True
            ;[1 1 1] South
            (if _btileinarray :!label _label_2
              (Utilities|CycleCounter (LocalVariables|GetL_CycleCounter) 4
                (:True
                  ;[1 1 1] East
                  (if _btileinarray_4 :!label _label_3
                    (Utilities|CycleCounter (LocalVariables|GetL_CycleCounter) 4
                      (:True
                        ;[1 1 1] West
                        (if _btileinarray_2 :!label _label_4
                          (Utilities|CycleCounter (LocalVariables|GetL_CycleCounter) 4
                            (:True
                              (goto _label))
                            (:False
                              (Variables|Default|SetbCurrentFreeSide? false :!label _label_5)))
                          (else
                            (CallFunction|AddBridge&PathTile _pathtile_2 _bridgetile_2))))
                      (:False
                        (goto _label_5)))
                    (else
                      (CallFunction|AddBridge&PathTile _pathtile_4 _bridgetile_4))))
                (:False
                  (goto _label_5)))
              (else
                (CallFunction|AddBridge&PathTile _pathtile _bridgetile))))
          (:False
            (goto _label_5)))
        (else
          (CallFunction|AddBridge&PathTile _pathtile_3 _bridgetile_3))))
    (:1
      (goto _label_3))
    (:2
      (goto _label_2))
    (:3
      (goto _label_4)))
  (return))

(fn BackTrack
  (bind _arrayelement (Utilities|ForEachLoopwithBrakRev (Variables|Default|GetPathTiles) :!label _label)
    (:LoopBody
      (if (not (Utilities|Array|ContainsItem (Variables|Default|GetCheckedTiles) _arrayelement))
        (Variables|Default|SetCurrentTile _arrayelement)
        (goto _label Break)))))

(fn PopulateWalls
  (bind _size (Variables|Default|GetSize))
  (for _index (range 0 (- (* _size _size) 1))
    (if (not (Utilities|CheckTileArrays _index))
      (Utilities|Array|Add (LocalVariables|GetAllWalls) _index)))
  (for (_array_element _array_index) (LocalVariables|GetAllWalls)
    (if (== (Math|Integer|%(Integer) _array_index 10) 3)
      (Utilities|Array|Add (Variables|Default|GetSandWallTiles) _array_element)
      (elif (== (Math|Integer|%(Integer) _array_index 10) 7)
        (Utilities|Array|Add (Variables|Default|GetBushWallTiles) _array_element)
        (else
          (Utilities|Array|Add (Variables|Default|GetNormalWallTiles) _array_element))))))